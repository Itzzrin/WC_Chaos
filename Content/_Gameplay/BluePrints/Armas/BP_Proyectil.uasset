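; BP_Proyectil is a weapon projectile that triggers a reaction in problem NPCs it hits.
; On spawn it checks the player's Arma2 flag and, if set, activates its Rayo component.
; A Sphere hit destroys the projectile, then passes any BP_NpcProblemas hit to VerificarNPC.
; VerificarNPC calls the NPC's FuncionPelea only when its blackboard BehaviorType matches one specific enum value.
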(event `self.ReceiveBeginPlay`
  (bind _asbp_player (cast `/Game/_Gameplay/Characters/BP_Player` (`GameplayStatics.GetPlayerCharacter` 0)))
  (if (`/Game/_Gameplay/Characters/BP_Player.Arma2` _asbp_player)
    (`ActorComponent.Activate` (`self.Rayo`) false)))

(event `self.Sphere.OnComponentHit`
  (params (HitComponent :type "PrimitiveComponent Object Reference") (OtherActor :type "Actor Object Reference") (OtherComp :type "PrimitiveComponent Object Reference") (NormalImpulse :type "Vector Structure") (Hit :type "HitResult Structure (by ref)"))
  (`self.K2_DestroyActor`)
  (bind _asbp_npc_problemas (cast `/Game/_Gameplay/IA/NPC_Problemas/BP_NpcProblemas` OtherActor))
  (`self.verificarNPC` _asbp_npc_problemas))

(fn `UserConstructionScript`)

(fn `verificarNPC`
  (params (`Hit Actor` :type "Actor Object Reference"))
  (if (== (`BlackboardComponent.GetValueAsEnum` (`AIBlueprintHelperLibrary.GetBlackboard` `Hit Actor`) "BehaviorType") 2)
    (bind _asbp_npc_problemas (cast `/Game/_Gameplay/IA/NPC_Problemas/BP_NpcProblemas` `Hit Actor`))
    (`/Game/_Gameplay/IA/NPC_Problemas/BP_NpcProblemas.funcionPelea` _asbp_npc_problemas)))