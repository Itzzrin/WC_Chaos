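; BP_Sky is a sky actor that runs a looping day-night cycle.
; Each Tick advances a Time value by frame delta divided by TimeDilation and resets it to zero after 240.
; Time maps to a full pitch rotation of the sun directional light, with the moon light offset 180 degrees opposite.
; A float curve sampled at Time sets the exponential height fog density across the cycle.
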(event `self.ReceiveTick`
  (params (DeltaSeconds :type "Float (single-precision)"))
  (bind _output_get (set `self.Time` (+ (/ DeltaSeconds (`self.TimeDilation`)) (`self.Time`))))
  (if (> _output_get 240.0)
    (set `self.Time` 0.0)
    (else
      (`SceneComponent.K2_SetRelativeRotation` (`self.DirectionalLight`) (`KismetMathLibrary.MakeRotator` 0.0 (* (/ (`self.Time`) 240.0) 360.0)) false false)
      (`SceneComponent.K2_SetRelativeRotation` (`self.DirectionalLight_Moon`) (`KismetMathLibrary.MakeRotator` 0.0 (+ (* (/ (`self.Time`) 240.0) 360.0) 180.0)) false false)
      (`ExponentialHeightFogComponent.SetFogDensity` (`self.ExponentialHeightFog`) (`CurveFloat.GetFloatValue` (`self.Curve`) (`self.Time`))))))

(fn `UserConstructionScript`)