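; Level manager that runs the lobby and three levels, handling teleports, cinematics, HUD widget, tagged-actor toggling and NPC spawning.
; Tick fills the lobby, keeps a spline-following queue NPC in level 1, and starts spawning in later levels after cinematics.
; Levels 2-3 use self-rescheduling timers for capped problem and background NPCs.
; Behaviour is random unless countdown equals 50 with player quotas unmet; fighters spawn as blackboard-linked pairs.
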(event `self.ReceiveBeginPlay`
  (bind _asbp_player (cast `/Game/_Gameplay/Characters/BP_Player` (`GameplayStatics.GetPlayerCharacter` 0)))
  (set `self.As BP Player` _asbp_player))

(event `self.ReceiveTick`
  (params (DeltaSeconds :type "Float (single-precision)"))
  (bind _nivel (`self.Nivel`))
  (bind _nivel_2 (`self.Nivel`))
  (if (or (== _nivel_2 0) (== _nivel_2 1))
    (if (== _nivel 1)
      (`/Engine/EditorBlueprintResources/StandardMacros.IsValid` (`self.CurrentNPC`)
        (:`Is Not Valid`
          (`self.spawnNPCfila`)))
      (elif (== _nivel 0)
        (if (< (`self.lobbyNPC`) 8)
          (`KismetSystemLibrary.Delay` 3.0)
          (`|SpawnActorFromClass` "/Game/_Gameplay/IA/NPC_Normal/BP_Npc.BP_Npc_C" (`KismetMathLibrary.MakeTransform` (`KismetArrayLibrary.Array_Random` (`self.Random Locations`))) "AlwaysSpawn" "OverrideRootScale" null null)
          (`/Engine/EditorBlueprintResources/StandardMacros.IncrementInt` (`self.lobbyNPC`)))))
    (elif (and (`self.cinematicaAcabo`) (not (`self.EmpezarSpawnear`)))
      (`self.spawnNPCNvl2`)
      (set `self.EmpezarSpawnear` true)
      (`KismetSystemLibrary.PrintString` "Empieza a spawnear"))))

(event `Lobby`
  (`|ExecutionSequence`
    (:`then_0`
      (bind _outactors (`GameplayStatics.GetAllActorsWithTag` "Lvl1"))
      (for _array_element _outactors
        (`self.SetActorHiddenInGame` _array_element false)
        (`self.SetActorEnableCollision` _array_element true)))
    (:`then_1`
      (bind _outactors_2 (`GameplayStatics.GetAllActorsWithTag` "Pared1"))
      (for _array_element_2 _outactors_2
        (`self.SetActorEnableCollision` _array_element_2 false)))))

(event `OnFinished_Event`
  (set `self.cinematicaAcabo` true))

(event `EmpezarNvl1`
  (bind (_tplvl1_location _tplvl1_rotation) (`KismetMathLibrary.BreakTransform` (`self.TpLvl1`)))
  (`|ExecutionSequence`
    (:`then_0`
      (bind (_outactor _returnvalue) (`LevelSequencePlayer.CreateLevelSequencePlayer` "/Game/_Core/Cinematicas/CinematicaPrimerNvl.CinematicaPrimerNvl"))
      (bind _output_get (set `self.cinematica` _returnvalue))
      (add `MovieSceneSequencePlayer.OnFinished` _output_get (delegate `OnFinished_Event`))
      (`MovieSceneSequencePlayer.Play` _output_get)
      (`MovieSceneSequencePlayer.Play` _returnvalue)
      (`self.K2_SetActorLocationAndRotation` (`GameplayStatics.GetPlayerCharacter` 0) _tplvl1_location _tplvl1_rotation false false)
      (`|ExecutionSequence`
        (:`then_0`
          (bind _outactors (`GameplayStatics.GetAllActorsWithTag` "Lvl1"))
          (for _array_element _outactors
            (`self.SetActorHiddenInGame` _array_element true)
            (`self.SetActorEnableCollision` _array_element false)))
        (:`then_1`
          (bind _outactors_2 (`GameplayStatics.GetAllActorsWithTag` "Pared1"))
          (for _array_element_2 _outactors_2
            (`self.SetActorEnableCollision` _array_element_2 true))
          (bind _returnvalue_2 (`|CreateWidget` "/Game/_Core/UI/WBP_BARRA.WBP_BARRA_C"))
          (`UserWidget.AddToViewport` _returnvalue_2 0)
          (set `self.WBP Nivel` _returnvalue_2))))
    (:`then_1`
      (`self.spawnNPCfila`))))

(event `spawnNPCfila`
  (bind _returnvalue (`GameplayStatics.GetActorOfClass` "/Game/_Gameplay/IA/NPC_Fila/BP_Spline.BP_Spline_C"))
  (bind _returnvalue_2 (`|SpawnActorFromClass` "/Game/_Gameplay/IA/NPC_Fila/BP_NpcFila.BP_NpcFila_C" (`KismetMathLibrary.MakeTransform` (`NavigationSystemV1.K2_GetRandomReachablePointInRadius` (`KismetMathLibrary.MakeVector` 2043.329924 11527.622636 106.750001) 350.0 null null)) "AlwaysSpawn" "OverrideRootScale" null _returnvalue null))
  (set `self.CurrentNPC` _returnvalue_2))

(event `EmpezarNvl2`
  (bind (_tplvl2_location _tplvl2_rotation) (`KismetMathLibrary.BreakTransform` (`self.TpLvl2`)))
  (`self.SetParametros`)
  (`self.K2_SetActorLocationAndRotation` (`GameplayStatics.GetPlayerCharacter` 0) _tplvl2_location _tplvl2_rotation false false)
  (`|ExecutionSequence`
    (:`then_1`
      (bind _outactors (`GameplayStatics.GetAllActorsWithTag` "Lvl1"))
      (for _array_element _outactors
        (`self.SetActorEnableCollision` _array_element true))
      (bind _returnvalue (`|CreateWidget` "/Game/_Core/UI/WBP_BARRA.WBP_BARRA_C"))
      (`UserWidget.AddToViewport` _returnvalue 0)
      (set `self.WBP Nivel` _returnvalue))))

(event `spawnNPCNvl2`
  (if (< (`self.numNPC`) (`self.maxNPC`))
    (`self.CalcularTiempoSpawn`)
    (else
      (set `self.SpawnTimerH` 0.0))))

(event `OnFinished_Event_0`
  (set `self.cinematicaAcabo` true))

(event `SetParametros`
  (switch `int` (`self.Nivel`)
    (:`2`
      (set `self.AllRandomLocations` (`self.RandomLocationsLvl2`))
      (set `self.minSpawnTime` 5.0)
      (set `self.maxSpawnTime` 10.0)
      (set `self.maxNPC` 8)
      (set `self.numDetenidos` 1)
      (set `self.num Mochilas` 6)
      (set `self.numPeleador` 2)
      (set `self.maxBots` 6)
      (bind (_outactor _returnvalue) (`LevelSequencePlayer.CreateLevelSequencePlayer` "/Game/_Core/Cinematicas/CinematicaNvl3.CinematicaNvl3"))
      (bind _output_get (set `self.cinematica` _returnvalue))
      (add `MovieSceneSequencePlayer.OnFinished` _returnvalue (delegate `OnFinished_Event_0`))
      (`MovieSceneSequencePlayer.Play` _output_get))
    (:`3`
      (set `self.AllRandomLocations` (`self.RandomLocationsLvl3`))
      (set `self.minSpawnTime` 5.0)
      (set `self.maxSpawnTime` 15.0)
      (set `self.maxNPC` 14)
      (set `self.numDetenidos` 2)
      (set `self.num Mochilas` 10)
      (set `self.numPeleador` 4)
      (bind _outactors (`GameplayStatics.GetAllActorsWithTag` "Lvl3"))
      (for _array_element _outactors
        (`self.SetActorHiddenInGame` _array_element false))
      (set `self.maxBots` 10)
      (bind (_outactor_2 _returnvalue_2) (`LevelSequencePlayer.CreateLevelSequencePlayer` "/Game/_Core/Cinematicas/CinematicaNvl2.CinematicaNvl2"))
      (bind _output_get_2 (set `self.cinematica` _returnvalue_2))
      (add `MovieSceneSequencePlayer.OnFinished` _returnvalue_2 (delegate `OnFinished_Event_1`))
      (`MovieSceneSequencePlayer.Play` _output_get_2)))
  (`self.spawnNormalNPCC`))

(event `OnFinished_Event_1`
  (set `self.cinematicaAcabo` true))

(fn `CalcularTiempoSpawn`
  (locals (SpawnTime :type "Float (double-precision)"))
  (bind _output_get (set `local.SpawnTime` (`KismetMathLibrary.RandomFloatInRange` (`self.minSpawnTime`) (`self.maxSpawnTime`))))
  (`KismetSystemLibrary.K2_SetTimer` null "SpawnearNPC" _output_get))

(fn `normalesFondo`
  (params (Location :type "Vector Structure"))
  (`|SpawnActorFromClass` "/Game/_Gameplay/IA/NPC_Problemas/BP_NpcProblemas.BP_NpcProblemas_C" (`KismetMathLibrary.MakeTransform` Location) "AlwaysSpawn" "OverrideRootScale" null "NewEnumerator0" null)
  (bind _result (`/Engine/EditorBlueprintResources/StandardMacros.IncrementInt` (`self.normalNPC`))
    (:`  `
      (set `self.normalNPC` _result)
      (`KismetSystemLibrary.K2_SetTimer` null "spawnNormalNPCC" 5.0))))

(fn `NPCcorredor`
  (locals (RandomLocations :type "Array of Vector Structure"))
  (bind _returnvalue (`|SpawnActorFromClass` "/Game/_Gameplay/IA/NPC_Problemas/BP_NpcProblemas.BP_NpcProblemas_C" (`KismetMathLibrary.MakeTransform` (`KismetArrayLibrary.Array_Random` (`local.RandomLocations`))) "AlwaysSpawn" "OverrideRootScale" null "NewEnumerator3" null))
  (set `/Game/_Gameplay/IA/NPC_Problemas/BP_NpcProblemas.BehaviorType` "NewEnumerator3" _returnvalue)
  (bind _returnvalue_2 (`GameplayStatics.SpawnSound2D` "/Game/_Core/Audios/ALERT-WARNING-SOUND-EFFECT-NO-COPYRIGHT-BAROGS-GAMING.ALERT-WARNING-SOUND-EFFECT-NO-COPYRIGHT-BAROGS-GAMING" 1.0 1.0 0.0 null))
  (set `/Game/_Gameplay/IA/NPC_Problemas/BP_NpcProblemas.Sonido` _returnvalue_2 _returnvalue)
  (`self.spawnNPCNvl2`))

(fn `NPChumo`
  (locals (RandomElegido :type "Array of Vector Structure"))
  (switch `int` (`self.Nivel`)
    (:`2`
      (set `local.RandomElegido` (`self.RandomLocationsLvl2`) :!label _label))
    (:`3`
      (if (== (`KismetMathLibrary.RandomIntegerInRange` 1 2) 1)
        (goto _label)
        (else
          (set `local.RandomElegido` (`self.RandomLocationsLvl3`))))))
  (bind _returnvalue (`|SpawnActorFromClass` "/Game/_Gameplay/IA/NPC_Problemas/BP_NpcProblemas.BP_NpcProblemas_C" (`KismetMathLibrary.MakeTransform` (`KismetArrayLibrary.Array_Random` (`local.RandomElegido`))) "AlwaysSpawn" "OverrideRootScale" null "NewEnumerator4" null))
  (set `/Game/_Gameplay/IA/NPC_Problemas/BP_NpcProblemas.BehaviorType` "NewEnumerator4" _returnvalue)
  (`self.spawnNPCNvl2`))

(fn `NPCmochila`
  (locals (RandomElegido :type "Array of Vector Structure"))
  (switch `int` (`self.Nivel`)
    (:`2`
      (set `local.RandomElegido` (`self.RandomLocationsLvl2`) :!label _label))
    (:`3`
      (if (== (`KismetMathLibrary.RandomIntegerInRange` 1 2) 1)
        (goto _label)
        (else
          (set `local.RandomElegido` (`self.RandomLocationsLvl3`))))))
  (bind _returnvalue (`|SpawnActorFromClass` "/Game/_Gameplay/IA/NPC_Problemas/BP_NpcProblemas.BP_NpcProblemas_C" (`KismetMathLibrary.MakeTransform` (`KismetArrayLibrary.Array_Random` (`local.RandomElegido`))) "AlwaysSpawn" "OverrideRootScale" null "NewEnumerator1" null))
  (set `/Game/_Gameplay/IA/NPC_Problemas/BP_NpcProblemas.BehaviorType` "NewEnumerator1" _returnvalue)
  (`self.spawnNPCNvl2`))

(fn `NPCnormal`
  (locals (RandodmElegido :type "Array of Vector Structure"))
  (switch `int` (`self.Nivel`)
    (:`2`
      (set `local.RandodmElegido` (`self.RandomLocationsLvl2`) :!label _label))
    (:`3`
      (if (== (`KismetMathLibrary.RandomIntegerInRange` 1 2) 1)
        (goto _label)
        (else
          (set `local.RandodmElegido` (`self.RandomLocationsLvl3`))))))
  (bind _returnvalue (`|SpawnActorFromClass` "/Game/_Gameplay/IA/NPC_Problemas/BP_NpcProblemas.BP_NpcProblemas_C" (`KismetMathLibrary.MakeTransform` (`KismetArrayLibrary.Array_Random` (`local.RandodmElegido`))) "AlwaysSpawn" "OverrideRootScale" null "NewEnumerator0" null))
  (set `/Game/_Gameplay/IA/NPC_Problemas/BP_NpcProblemas.BehaviorType` "NewEnumerator0" _returnvalue)
  (`self.spawnNPCNvl2`))

(fn `NPCpeleador`
  (locals (randomElegido :type "Array of Vector Structure"))
  (bind _npcporspawnear (`self.npcPorSpawnear`))
  (if (!= (`self.Nivel`) 2)
    (if (== (`KismetMathLibrary.RandomIntegerInRange` 1 2) 1)
      (set `local.randomElegido` (`self.RandomLocationsLvl2`))
      (else
        (set `local.randomElegido` (`self.RandomLocationsLvl3`))))
    (else
      (set `local.randomElegido` (`self.RandomLocationsLvl2`))))
  (bind _returnvalue (`|SpawnActorFromClass` "/Game/_Gameplay/IA/NPC_Problemas/BP_NpcProblemas.BP_NpcProblemas_C" (`KismetMathLibrary.MakeTransform` (`KismetArrayLibrary.Array_Random` (`local.randomElegido`))) "AlwaysSpawn" "OverrideRootScale" null "NewEnumerator2" null))
  (set `self.npcPorSpawnear` _returnvalue)
  (set `/Game/_Gameplay/IA/NPC_Problemas/BP_NpcProblemas.BehaviorType` "NewEnumerator2" _returnvalue)
  (bind _returnvalue_2 (`|SpawnActorFromClass` "/Game/_Gameplay/IA/NPC_Problemas/BP_NpcProblemas.BP_NpcProblemas_C" (`KismetMathLibrary.MakeTransform` (`KismetArrayLibrary.Array_Random` (`local.randomElegido`))) "AlwaysSpawn" "OverrideRootScale" null "NewEnumerator2" null))
  (set `/Game/_Gameplay/IA/NPC_Problemas/BP_NpcProblemas.BehaviorType` "NewEnumerator2" _npcporspawnear)
  (`BlackboardComponent.SetValueAsObject` (`AIBlueprintHelperLibrary.GetBlackboard` _returnvalue_2) "FightPartner" _npcporspawnear)
  (set `/Game/_Gameplay/IA/NPC_Problemas/BP_NpcProblemas.FightPartner` _npcporspawnear _returnvalue_2)
  (bind _result (`/Engine/EditorBlueprintResources/StandardMacros.IncrementInt` (`self.numNPC`))
    (:`  `
      (set `self.numNPC` _result)
      (`self.spawnNPCNvl2`))))

(fn `SpawnearNPC`
  (`|ExecutionSequence`
    (:`then_0`
      (if (< (`self.numNPC`) (`self.maxNPC`))
        (bind _asbp_player (cast `/Game/_Gameplay/Characters/BP_Player` (`GameplayStatics.GetPlayerCharacter` 0)))
        (set `self.As BP Player` _asbp_player)
        (if (and (== (`/Game/_Core/UI/WBP_BARRA.CountDown` (`self.WBP Nivel`)) 50.0) (< (`/Game/_Gameplay/Characters/BP_Player.Detenidos` (`self.As BP Player`)) (`self.numDetenidos`)))
          (set `self.BT` "NewEnumerator3")
          (elif (and (== (`/Game/_Core/UI/WBP_BARRA.CountDown` (`self.WBP Nivel`)) 50.0) (< (`/Game/_Gameplay/Characters/BP_Player.Mochilas` (`self.As BP Player`)) (`self.num Mochilas`)))
            (set `self.BT` "NewEnumerator1")
            (elif (and (== (`/Game/_Core/UI/WBP_BARRA.CountDown` (`self.WBP Nivel`)) 50.0) (< (`/Game/_Gameplay/Characters/BP_Player.Peleas` (`self.As BP Player`)) (`self.numPeleador`)))
              (set `self.BT` "NewEnumerator2")
              (else
                (set `self.BT` (cast `/Game/_Gameplay/IA/NPC_Problemas/E_NpcTipo` (`KismetMathLibrary.Conv_IntToByte` (`KismetMathLibrary.RandomIntegerInRange` 0 4))))))))))
    (:`then_1`
      (bind _result (`/Engine/EditorBlueprintResources/StandardMacros.IncrementInt` (`self.numNPC`))
        (:`  `
          (set `self.numNPC` _result)
          (switch `/Game/_Gameplay/IA/NPC_Problemas/E_NpcTipo` (`self.BT`)
            (:`NewEnumerator0`
              (`self.NPCmochila`))
            (:`NewEnumerator1`
              (`self.NPCmochila`))
            (:`NewEnumerator2`
              (`self.NPCpeleador`))
            (:`NewEnumerator3`
              (`self.NPCcorredor`))
            (:`NewEnumerator4`
              (`self.NPChumo`))))))))

(fn `spawnNormalNPCC`
  (if (<= (`self.normalNPC`) (`self.maxBots`))
    (switch `int` (`self.Nivel`)
      (:`2`
        (`self.normalesFondo` (`KismetArrayLibrary.Array_Random` (`self.RandomLocationsLvl2`)) :!label _label))
      (:`3`
        (if (== (`KismetMathLibrary.RandomIntegerInRange` 1 2) 1)
          (goto _label)
          (else
            (`self.normalesFondo` (`KismetArrayLibrary.Array_Random` (`self.RandomLocationsLvl3`)))))))))

(fn `UserConstructionScript`)