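; Player inventory component that stores item stacks in a fixed-size slot array and handles item interaction and the pausing inventory menu.
; A per-tick camera sphere trace sets the look-at target; the interact input messages its ItemDataComponent and reloads the widget.
; Adding fills stacks up to DataTable limits before using empty slots; removal is an empty stub.
; Contents load from GameInstance save data on BeginPlay, with a function to save them to disk.
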(event `self.ReceiveBeginPlay`
  (`self.LoadSaveInv`)
  (bind _returnvalue (`|CreateWidget` "/Game/_Core/UI/WBP_INVENTARIO.WBP_INVENTARIO_C"))
  (set `self.Inventory` _returnvalue)
  (`KismetArrayLibrary.Array_Resize` (`self.Content`) (`self.InventorySize`))
  (`/Game/_Core/UI/WBP_INVENTARIO.LoadInventory` (`self.Inventory`) self))

(event `EnhancedInput|/Game/_Gameplay/Input/Actions/IA_Inventario`
  (params (ActionValue :type Boolean) (ElapsedSeconds :type "Float (double-precision)") (TriggeredSeconds :type "Float (double-precision)") (InputAction :type "InputAction Object Reference" :default "/Game/_Gameplay/Input/Actions/IA_Inventario.IA_Inventario"))
  (bind _returnvalue (`GameplayStatics.GetPlayerController` 0))
  (bind _inventory (`self.Inventory`))
  (bind (_sizex _sizey) (`PlayerController.GetViewportSize` _returnvalue))
  (:`Started`
    (if (`Widget.IsVisible` (`self.Inventory`))
      (`Widget.RemoveFromParent` _inventory)
      (`GameplayStatics.SetGamePaused` false)
      (set `PlayerController.bShowMouseCursor` false (`GameplayStatics.GetPlayerController` 0))
      (else
        (`UserWidget.AddToViewport` _inventory 0)
        (`GameplayStatics.SetGamePaused` true)
        (set `PlayerController.bShowMouseCursor` true _returnvalue)
        (`PlayerController.SetMouseLocation` _returnvalue (`KismetMathLibrary.FTrunc` (`KismetMathLibrary.SafeDivide` (`KismetMathLibrary.Conv_IntToDouble` _sizex) 2.0)) (`KismetMathLibrary.FTrunc` (`KismetMathLibrary.SafeDivide` (`KismetMathLibrary.Conv_IntToDouble` _sizey) 2.0)))))))

(event `self.ReceiveTick`
  (params (DeltaSeconds :type "Float (single-precision)"))
  (`self.InteractionTrace`))

(event `EnhancedInput|/Game/_Gameplay/Input/Actions/IA_Interactuar`
  (params (ActionValue :type Boolean) (ElapsedSeconds :type "Float (double-precision)") (TriggeredSeconds :type "Float (double-precision)") (InputAction :type "InputAction Object Reference" :default "/Game/_Gameplay/Input/Actions/IA_Interactuar.IA_Interactuar"))
  (:`Started`
    (bind _lookatactor (`self.LookAtActor`)
      (:`then`
        (`self.Server_Interact` _lookatactor))
      (:`else`))))

(event `Server_Interact`
  (params (Target :type "Actor Object Reference"))
  (bind _returnvalue (`Actor.GetComponentByClass` Target "/Game/_Gameplay/BluePrints/Inventory/ItemDataComponent.ItemDataComponent_C"))
  (`/Engine/EditorBlueprintResources/StandardMacros.IsValid` _returnvalue
    (:`Is Valid`
      (message `/Game/_Gameplay/BluePrints/Inventory/I_InteractInterface.InteractWith` _returnvalue (cast `/Game/_Gameplay/Characters/BP_Player` (`self.GetOwner`) :!pure true))
      (`/Game/_Core/UI/WBP_INVENTARIO.LoadInventory` (`self.Inventory`) self))))

(event `Key|One`
  (params (Key :type "Key Structure"))
  (:`Pressed`
    (`self.DEBUG_Print`)))

(fn `AddToInventory`
  (params (ItemID :type Name) (Quantity :type Integer))
  (returns (Success :type Boolean) (QuantityRemaining :type Integer))
  (locals (LocalQuantityRemaining :type Integer) (Local_HasFailed :type Boolean))
  (set `local.LocalQuantityRemaining` Quantity)
  (while (and (> (`local.LocalQuantityRemaining`) 0) (not (`local.Local_HasFailed`)))
    (bind (_index _foundslot) (`self.FindSlot` (`local.ItemID`)))
    (if _foundslot
      (`self.AddToStack` _index 1)
      (`/Engine/EditorBlueprintResources/StandardMacros.DecrementInt` (`local.LocalQuantityRemaining`))
      (elif (`self.AnyEmptySlot`)
        (bind _success (`self.CreateNewStack` (`local.ItemID`) 1))
        (if _success
          (`/Engine/EditorBlueprintResources/StandardMacros.DecrementInt` (`local.LocalQuantityRemaining`))
          (else
            (set `local.Local_HasFailed` true)))
        (else
          (set `local.Local_HasFailed` true)))))
  (return (not (`local.Local_HasFailed`)) (`local.LocalQuantityRemaining`)))

(fn `AddToStack`
  (params (Index :type Integer) (Quantity :type Integer))
  (bind (_output_itemid _output_quantity) (break `/Game/_Gameplay/BluePrints/Inventory/S_SlotStruct` (`|GetArrayItem` (`self.Content`) Index)))
  (`KismetArrayLibrary.Array_Set` (`self.Content`) Index (make `/Game/_Gameplay/BluePrints/Inventory/S_SlotStruct` _output_itemid (+ _output_quantity (`local.Quantity`)))))

(fn `AnyEmptySlot`
  (returns (HasEmptySlot :type Boolean) (EmptyIndex :type Integer))
  (for (_array_element _array_index) (`self.Content`)
    (if (== (`.Quantity_6_1E843D264E20B1D39B844AB692D50E95` (break `/Game/_Gameplay/BluePrints/Inventory/S_SlotStruct` _array_element)) 0)
      (return true _array_index)))
  (return false -1))

(fn `CreateNewStack`
  (params (ItemID :type Name) (Quantity :type Integer))
  (returns (Success :type Boolean))
  (bind (_hasemptyslot _emptyindex) (`self.AnyEmptySlot`))
  (if _hasemptyslot
    (`KismetArrayLibrary.Array_Set` (`self.Content`) _emptyindex (make `/Game/_Gameplay/BluePrints/Inventory/S_SlotStruct` (`local.ItemID`) (`local.Quantity`)))
    (return true)
    (else
      (return false))))

(fn `DEBUG_Print`
  (for (_array_element _array_index) (`self.Content`)
    (bind (_itemid _quantity) (break `/Game/_Gameplay/BluePrints/Inventory/S_SlotStruct` _array_element))
    (`KismetSystemLibrary.PrintString` (`KismetStringLibrary.Concat_StrStr` (`KismetStringLibrary.Conv_IntToString` _array_index) ":" (`KismetStringLibrary.Conv_NameToString` _itemid) "=" (`KismetStringLibrary.Conv_IntToString` _quantity)))))

(fn `FindSlot`
  (params (ItemID :type Name))
  (returns (Index :type Integer) (FoundSlot :type Boolean))
  (bind _itemid (`local.ItemID`))
  (for (_array_element _array_index) (`self.Content`)
    (bind (_itemid_2 _quantity) (break `/Game/_Gameplay/BluePrints/Inventory/S_SlotStruct` _array_element))
    (if (== _itemid_2 _itemid)
      (if (< _quantity (`self.GetMaxStackSize` _itemid))
        (return _array_index true))))
  (return -1 false))

(fn `GetMaxStackSize`
  (params (ItemID :type Name))
  (returns (StackSize :type Integer))
  (bind _returnvalue (`|GetDataTableRow` "/Game/_Gameplay/BluePrints/Inventory/ItemData.ItemData" ItemID)
    (:`then`
      (return (`.StackSize_14_642C28FF4AC8E580D99A0799E0BDBA06` (break `/Game/_Gameplay/BluePrints/Inventory/S_ItemStruct` _returnvalue))))
    (:`RowNotFound`
      (return -1))))

(fn `InteractionTrace`
  (bind _returnvalue (`GameplayStatics.GetPlayerCameraManager` 0))
  (bind _returnvalue_2 (`Actor.K2_GetActorLocation` _returnvalue))
  (bind (_outhit _returnvalue_3) (`KismetSystemLibrary.SphereTraceSingle` _returnvalue_2 (+ _returnvalue_2 (* (`Actor.GetActorForwardVector` _returnvalue) (`self.InteractionRange`))) 15.0 "TraceTypeQuery3" false (`|MakeArray` (`self.GetOwner`))))
  (if _returnvalue_3
    (bind (_bblockinghit _binitialoverlap _time _distance _location _impactpoint _normal _impactnormal _physmat _hitactor) (`GameplayStatics.BreakHitResult` _outhit))
    (if (!= _hitactor (`self.LookAtActor`))
      (bind _output_get (set `self.LookAtActor` _hitactor))
      (bind _msg (message `/Game/_Gameplay/BluePrints/Inventory/I_InteractInterface.LookAt` _output_get))
      (`KismetSystemLibrary.PrintString` (`KismetTextLibrary.Conv_TextToString` _msg)))
    (else
      (set `self.LookAtActor` null))))

(fn `LoadSaveInv`
  (bind _aswchaos_game_instance (cast `/Game/_Gameplay/BluePrints/SaveGame/WChaos_GameInstance` (`GameplayStatics.GetGameInstance`)))
  (set `self.Content` (`/Game/_Gameplay/BluePrints/SaveGame/SaveData_PlayerData.InventoryContent` (`/Game/_Gameplay/BluePrints/SaveGame/WChaos_GameInstance.As Save Data Player Data` _aswchaos_game_instance))))

(fn `RemoveFromInventory`)

(fn `SaveInventory`
  (bind _aswchaos_game_instance (cast `/Game/_Gameplay/BluePrints/SaveGame/WChaos_GameInstance` (`GameplayStatics.GetGameInstance`)))
  (bind _as_save_data_player_data (`/Game/_Gameplay/BluePrints/SaveGame/WChaos_GameInstance.As Save Data Player Data` _aswchaos_game_instance))
  (set `/Game/_Gameplay/BluePrints/SaveGame/SaveData_PlayerData.InventoryContent` (`self.Content`) _as_save_data_player_data)
  (`GameplayStatics.SaveGameToSlot` _as_save_data_player_data "MyData"))