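; Problem NPC that the player can intervene on, acting as a backpack carrier, fighter, runner or smoker according to BehaviorType.
; BeginPlay passes the type to the Blackboard and picks a random mesh and AnimBP from a DataTable.
; Box overlap sets player interaction flags by type, some gated on CurrentState, and clears them on exit.
; Resolution functions change Blackboard state, hide the indicator and update player stats, inventory or level NPC count.
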(event `self.ReceiveBeginPlay`
  (bind _returnvalue (`AIBlueprintHelperLibrary.GetBlackboard` self))
  (bind _mesh (`self.Mesh`))
  (`BlackboardComponent.SetValueAsEnum` _returnvalue "BehaviorType" (`self.BehaviorType`))
  (`BlackboardComponent.SetValueAsObject` _returnvalue "SelfActor" self)
  (bind _returnvalue_2 (`|GetDataTableRow` "/Game/_Gameplay/Characters/ModelosNPC/DT_Meshes.DT_Meshes" (`|GetArrayItem` (`self.meshes`) (`KismetMathLibrary.RandomInteger` 3)))
    (:`then`
      (`SkeletalMeshComponent.SetSkeletalMeshAsset` _mesh (break `/Game/_Gameplay/Characters/ModelosNPC/S_Meshes` _returnvalue_2))
      (`SkeletalMeshComponent.SetAnimInstanceClass` _mesh (`.AnimationBP_5_8006F21843A9F581EC64F6AD8DA1ACCC` (break `/Game/_Gameplay/Characters/ModelosNPC/S_Meshes` _returnvalue_2))))))

(event `self.PawnSensing.OnSeePawn`
  (params (Pawn :type "Pawn Object Reference"))
  (cast `/Game/_Gameplay/Characters/BP_Player` Pawn))

(event `self.Box.OnComponentBeginOverlap`
  (params (OverlappedComponent :type "PrimitiveComponent Object Reference") (OtherActor :type "Actor Object Reference") (OtherComp :type "PrimitiveComponent Object Reference") (OtherBodyIndex :type Integer) (bFromSweep :type Boolean) (SweepResult :type "HitResult Structure (by ref)"))
  (bind _as_bp_player (`self.As BP Player`))
  (bind _returnvalue (== (`BlackboardComponent.GetValueAsEnum` (`AIBlueprintHelperLibrary.GetBlackboard` self) "CurrentState") 2))
  (bind _asbp_player (cast `/Game/_Gameplay/Characters/BP_Player` OtherActor))
  (bind _output_get (set `self.As BP Player` _asbp_player))
  (if (`/Game/_Gameplay/Characters/BP_Player.Ocupado` _output_get)
    (set `/Game/_Gameplay/Characters/BP_Player.Ocupado` true _output_get))
  (set `/Game/_Gameplay/Characters/BP_Player.NpcReference` self _output_get)
  (switch `/Game/_Gameplay/IA/NPC_Problemas/E_NpcTipo` (`self.BehaviorType`)
    (:`NewEnumerator1`
      (`self.funcionMochila`))
    (:`NewEnumerator2`
      (if _returnvalue
        (set `/Game/_Gameplay/Characters/BP_Player.puedeDetenerPelea` true _as_bp_player)))
    (:`NewEnumerator3`
      (set `/Game/_Gameplay/Characters/BP_Player.puedeDetenerCorredor` true _as_bp_player))
    (:`NewEnumerator4`
      (if _returnvalue
        (set `/Game/_Gameplay/Characters/BP_Player.puedeDetenerHumo` true _as_bp_player)))))

(event `self.Box.OnComponentEndOverlap`
  (params (OverlappedComponent :type "PrimitiveComponent Object Reference") (OtherActor :type "Actor Object Reference") (OtherComp :type "PrimitiveComponent Object Reference") (OtherBodyIndex :type Integer))
  (bind _as_bp_player (`self.As BP Player`))
  (bind _asbp_player (cast `/Game/_Gameplay/Characters/BP_Player` OtherActor))
  (set `/Game/_Gameplay/Characters/BP_Player.NpcReference` self _asbp_player)
  (set `/Game/_Gameplay/Characters/BP_Player.puedeAbrirMochila` false _as_bp_player)
  (set `/Game/_Gameplay/Characters/BP_Player.puedeDetenerCorredor` false _as_bp_player)
  (set `/Game/_Gameplay/Characters/BP_Player.puedeDetenerHumo` false _as_bp_player)
  (set `/Game/_Gameplay/Characters/BP_Player.puedeDetenerPelea` false _as_bp_player))

(fn `funcionCorredor`
  (bind _as_bp_player (`self.As BP Player`))
  (bind _sonido (`self.Sonido`))
  (bind _result (`/Engine/EditorBlueprintResources/StandardMacros.IncrementInt` (`/Game/_Gameplay/Characters/BP_Player.Detenidos` _as_bp_player))
    (:`  `
      (set `/Game/_Gameplay/Characters/BP_Player.Detenidos` _result _as_bp_player)
      (set `/Game/_Gameplay/Characters/BP_Player.Vida` (+ (`/Game/_Gameplay/Characters/BP_Player.Vida` _as_bp_player) 5.0) _as_bp_player)
      (set `/Game/_Gameplay/Characters/BP_Player.puedeDetenerCorredor` false _as_bp_player)
      (bind _returnvalue (`GameplayStatics.GetActorOfClass` "/Game/_Gameplay/BluePrints/Niveles/BP_Niveles.BP_Niveles_C"))
      (bind _result_2 (`/Engine/EditorBlueprintResources/StandardMacros.DecrementInt` (`/Game/_Gameplay/BluePrints/Niveles/BP_Niveles.numNPC` _returnvalue))
        (:`  `
          (set `/Game/_Gameplay/BluePrints/Niveles/BP_Niveles.numNPC` _result_2 _returnvalue)
          (`BlackboardComponent.SetValueAsEnum` (`AIBlueprintHelperLibrary.GetBlackboard` self) "CurrentState" 6)
          (`SceneComponent.SetHiddenInGame` (`self.img`) true false)
          (`ActorComponent.Activate` (`self.tierra`) false)
          (`AudioComponent.SetPaused` _sonido true)
          (`ActorComponent.K2_DestroyComponent` _sonido))))))

(fn `funcionHumo`
  (set `/Game/_Gameplay/Characters/BP_Player.puedeDetenerHumo` false (`self.As BP Player`))
  (bind _returnvalue (`GameplayStatics.GetActorOfClass` "/Game/_Gameplay/BluePrints/Niveles/BP_Niveles.BP_Niveles_C"))
  (bind _result (`/Engine/EditorBlueprintResources/StandardMacros.DecrementInt` (`/Game/_Gameplay/BluePrints/Niveles/BP_Niveles.numNPC` _returnvalue))
    (:`  `
      (set `/Game/_Gameplay/BluePrints/Niveles/BP_Niveles.numNPC` _result _returnvalue)
      (`BlackboardComponent.SetValueAsEnum` (`AIBlueprintHelperLibrary.GetBlackboard` self) "CurrentState" 6)
      (set `self.isFlare` false)
      (`SceneComponent.SetHiddenInGame` (`self.img`) true false)
      (`/Game/_Gameplay/BluePrints/Inventory/InventorySystem.ObjetoConfiscado` (`/Game/_Gameplay/Characters/BP_Player.InventorySystem` (`self.As BP Player`)) (make `DataTableRowHandle` "/Game/_Gameplay/BluePrints/Inventory/ItemData.ItemData" "Flare") 1))))

(fn `funcionMochila`
  (bind _as_bp_player (`self.As BP Player`))
  (if (== (`BlackboardComponent.GetValueAsEnum` (`AIBlueprintHelperLibrary.GetBlackboard` self) "CurrentState") 2)
    (set `/Game/_Gameplay/Characters/BP_Player.puedeAbrirMochila` true _as_bp_player)
    (set `/Game/_Gameplay/Characters/BP_Player.NpcReference` self _as_bp_player)))

(fn `funcionPelea`
  (locals (NewLocalVar :type "/Game/_Gameplay/Characters/BP_Player Object Reference"))
  (bind _newlocalvar (`local.NewLocalVar`))
  (bind _asbp_player (cast `/Game/_Gameplay/Characters/BP_Player` (`GameplayStatics.GetPlayerCharacter` 0)))
  (set `local.NewLocalVar` _asbp_player)
  (if (`/Game/_Gameplay/Characters/BP_Player.puedeDetenerPelea` _asbp_player)
    (`BlackboardComponent.SetValueAsEnum` (`AIBlueprintHelperLibrary.GetBlackboard` self) "CurrentState" 6 :!label _label)
    (`BlackboardComponent.SetValueAsEnum` (`AIBlueprintHelperLibrary.GetBlackboard` (`self.FightPartner`)) "CurrentState" 6)
    (set `/Game/_Gameplay/Characters/BP_Player.puedeDetenerPelea` false _newlocalvar)
    (bind _result (`/Engine/EditorBlueprintResources/StandardMacros.IncrementInt` (`/Game/_Gameplay/Characters/BP_Player.Peleas` _newlocalvar))
      (:`  `
        (set `/Game/_Gameplay/Characters/BP_Player.Peleas` _result _newlocalvar)
        (set `self.isFighting` false)
        (bind _asbp_npc_problemas (cast `/Game/_Gameplay/IA/NPC_Problemas/BP_NpcProblemas` (`self.FightPartner`)))
        (set `/Game/_Gameplay/IA/NPC_Problemas/BP_NpcProblemas.isFighting` false _asbp_npc_problemas)
        (`SceneComponent.SetHiddenInGame` (`self.img`) true false)
        (`SceneComponent.SetHiddenInGame` (`/Game/_Gameplay/IA/NPC_Problemas/BP_NpcProblemas.img` _asbp_npc_problemas) true false)))
    (elif (`/Game/_Gameplay/Characters/BP_Player.puedeDetenerPistola` _asbp_player)
      (goto _label))))

(fn `UserConstructionScript`)