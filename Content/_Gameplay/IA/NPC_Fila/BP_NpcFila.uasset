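; BP_NpcFila is an NPC, likely one standing in a queue, whose backpack the player can open when nearby.
; On BeginPlay it registers itself as the owner of its Path, which the NpcPath function exposes.
; A Box overlap lets BP_Player open the backpack and passes this NPC as the target.
; Leaving the box clears only the permission flag, keeping the NPC reference.
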(event `self.ReceiveBeginPlay`
  (set `/Game/_Gameplay/IA/NPC_Fila/BP_Spline.NpcOwner` self (`self.Path`)))

(event `self.Box.OnComponentBeginOverlap`
  (params (OverlappedComponent :type "PrimitiveComponent Object Reference") (OtherActor :type "Actor Object Reference") (OtherComp :type "PrimitiveComponent Object Reference") (OtherBodyIndex :type Integer) (bFromSweep :type Boolean) (SweepResult :type "HitResult Structure (by ref)"))
  (bind _asbp_player (cast `/Game/_Gameplay/Characters/BP_Player` OtherActor))
  (bind _output_get (set `self.As BP Player` _asbp_player))
  (set `/Game/_Gameplay/Characters/BP_Player.puedeAbrirMochila` true _output_get)
  (set `/Game/_Gameplay/Characters/BP_Player.npcMochila` self _output_get))

(event `self.Box.OnComponentEndOverlap`
  (params (OverlappedComponent :type "PrimitiveComponent Object Reference") (OtherActor :type "Actor Object Reference") (OtherComp :type "PrimitiveComponent Object Reference") (OtherBodyIndex :type Integer))
  (bind _asbp_player (cast `/Game/_Gameplay/Characters/BP_Player` OtherActor))
  (set `/Game/_Gameplay/Characters/BP_Player.puedeAbrirMochila` false _asbp_player))

(fn `NpcPath`
  (returns (Path :type "/Game/_Gameplay/IA/NPC_Fila/BP_Spline Object Reference"))
  (return (`self.Path`)))

(fn `UserConstructionScript`)